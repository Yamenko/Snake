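; Actor Blueprint that procedurally builds a rectangular zone in its construction script, sized by Collumn, Row and Padding.
; Two loops add manually attached child actors along the edges, with the column sides yawed 90 degrees.
; Each opposite edge mirrors the world location of the component just created.
; A nested loop fills the interior with a centred grid of flattened static meshes, lowered by half the padding.
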(event EventBeginPlay)

(event Collision|EventActorBeginOverlap
  (params (OtherActor :type Actor%20Object%20Reference)))

(event EventTick
  (params (DeltaSeconds :type Float%20%28single-precision%29)))

(fn ConstructionScript
  (bind _collumn (Variables|Default|Getcollumn))
  (bind _padding (Variables|Default|Getpadding))
  (bind _row (Variables|Default|Getrow))
  (bind _padding_2 (Variables|Default|Getpadding))
  (bind _padding_3 (Variables|Default|Getpadding))
  (bind _padding_4 (Variables|Default|Getpadding))
  (bind _collumn_2 (Variables|Default|Getcollumn))
  (Utilities|FlowControl|Sequence
    (:then_0
      (for _index (range 1 _collumn_2)
        (bind _returnvalue (AddComponent|AddChildActorComponent true (Math|Transform|MakeTransform (Math|Vector|MakeVector (- (- (* _index (Variables|Default|Getpadding)) (/ (* _collumn_2 _padding) 2.0)) (/ (Variables|Default|Getpadding) 2.0)) (/ (* (Variables|Default|Getrow) _padding) 2.0) 0.0) "0,90.000000, 0" "1,1,1")))
        (AddComponent|AddChildActorComponent true (Math|Transform|MakeTransform (Math|Vector|MakeVector (.x (Transformation|GetWorldLocation _returnvalue)) (* -1 (.y (Transformation|GetWorldLocation _returnvalue))) 0.0) "0,90.000000, 0" "1,1,1"))))
    (:then_1
      (for _index_2 (range 1 _row)
        (bind _returnvalue_2 (AddComponent|AddChildActorComponent true (Math|Transform|MakeTransform (Math|Vector|MakeVector (/ (* (Variables|Default|Getcollumn) _padding_4) 2.0) (- (- (* _index_2 (Variables|Default|Getpadding)) (/ (* _row _padding_4) 2.0)) (/ (Variables|Default|Getpadding) 2.0)) 0.0) "0, 0, 0" "1,1,1")))
        (AddComponent|AddChildActorComponent true (Math|Transform|MakeTransform (Math|Vector|MakeVector (* -1 (.x (Transformation|GetWorldLocation _returnvalue_2))) (.y (Transformation|GetWorldLocation _returnvalue_2)) 0.0) "0, 0, 0" "1,1,1"))))
    (:then_2
      (for _index_3 (range 1 (Variables|Default|Getrow))
        (for _index_4 (range 1 _collumn)
          (AddComponent|AddStaticMeshComponent false (Math|Transform|MakeTransform (Math|Vector|MakeVector (- (- (* _index_4 _padding_3) (/ (* _collumn _padding_3) 2.0)) (/ _padding_3 2.0)) (- (- (* _index_3 (Variables|Default|Getpadding)) (/ (* (Variables|Default|Getrow) (Variables|Default|Getpadding)) 2.0)) (/ _padding_2 2.0)) (* (/ _padding_2 2.0) -1.0)) "0, 0, 0" "1,1,0.200000")))))))